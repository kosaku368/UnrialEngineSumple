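; BP_Award is a character that ragdolls when damaged and spends a life from AwardGameInstace.
; On the first damage event it disables movement and simulates mesh physics.
; It then either decrements Life and expires after three seconds or, with no lives left, opens the End level after a delay.
; At BeginPlay in the End level, it turns its lights red if the game was not cleared.
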(event `self.ReceiveBeginPlay`
  (bind _returnvalue (`self.ChackClearDirecting`))
  (if _returnvalue
    (`LightComponent.SetLightColor` (`self.PointLight`) (struct :`R` 1.0 :`A` 1.0) true)
    (`LightComponent.SetLightColor` (`self.HeadLight`) (struct :`R` 1.0 :`A` 1.0) true)))

(event `self.ReceiveAnyDamage`
  (params (Damage :type "Float (single-precision)") (DamageType :type "DamageType Object Reference") (InstigatedBy :type "Controller Object Reference") (DamageCauser :type "Actor Object Reference"))
  (bind _mesh (`self.Mesh`))
  (bind _asaward_game_instace (cast `/Game/BP/AwardGameInstace` (`GameplayStatics.GetGameInstance`) :!pure true))
  (bind _life (`/Game/BP/AwardGameInstace.Life` _asaward_game_instace))
  (`/Engine/EditorBlueprintResources/StandardMacros.DoOnce` false
    (:`Completed`
      (`|ExecutionSequence`
        (:`then_0`
          ;[1 1 1] ラグドール処理
          (`CharacterMovementComponent.DisableMovement` (`self.CharacterMovement`))
          (`PrimitiveComponent.SetCollisionProfileName` _mesh "Ragdoll" true)
          (`PrimitiveComponent.SetSimulatePhysics` _mesh true))
        (:`then_1`
          ;[1 1 1] ライフ処理
          (if (> _life 0)
            (set `/Game/BP/AwardGameInstace.Life` (- _life 1) _asaward_game_instace)
            (`self.SetLifeSpan` 3.0)
            (else
              (`KismetSystemLibrary.Delay` 3.0)
              (`GameplayStatics.OpenLevel` "End"))))))))

(fn `ChackClearDirecting`
  (returns (ReturnValue :type Boolean))
  (bind _returnvalue (`GameplayStatics.GetCurrentLevelName` true))
  (return (and (`KismetStringLibrary.EqualEqual_StrStr` _returnvalue "End") (not (`/Game/BP/AwardGameInstace.IsClear` (cast `/Game/BP/AwardGameInstace` (`GameplayStatics.GetGameInstance`) :!pure true))))))

(fn `UserConstructionScript`)