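; Game mode for the Award game that runs stage streaming, player respawn, the play HUD and the run timer.
; When the pawn is destroyed, it spawns and possesses a new BP_Award at the PlayerStart and rebinds the destroy event.
; Stages are streamed levels; NextStage increments the number in the stage name, swaps levels and moves the pawn to the PlayerStart.
; BeginPlay resets AwardGameInstace stats, and a looping one-second timer counts minutes and seconds there, capped at 99:59.
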(event `self.ReceiveBeginPlay`
  (`self.RespawnEvent`)
  (`self.LoadStage`)
  (`self.CreateUi`)
  (`self.InitialGameInstance`)
  (`self.Time`))

(event `RespawnEvent`
  ;[1 1 1] リスポーン
  (add `self.OnDestroyed` (`GameplayStatics.GetPlayerPawn` 0) (delegate `RespawnAward`)))

(event `RespawnAward` :!signature `self.OnDestroyed`
  (params (DestroyedActor :type "Actor Object Reference"))
  ;[1 1 1] リスポーン
  (bind _returnvalue (`|SpawnActorFromClass` "/Game/BP/BP_Award.BP_Award_C" (`self.GetTransform` (`self.K2_FindPlayerStart` null)) "Undefined" "OverrideRootScale" null null))
  (`Controller.Possess` (`GameplayStatics.GetPlayerController` 0) _returnvalue)
  (`self.RespawnEvent`))

(event `LoadStage`
  ;[1 1 1] LoadStage
  (`GameplayStatics.LoadStreamLevel` (`self.StageName`) true true)
  (`self.SetAwardTransform`))

(event `NextStage`
  (bind _stagename (`self.StageName`))
  (bind _returnvalue (`KismetStringLibrary.Conv_NameToString` _stagename))
  ;[1 1 1] NextStage
  (`GameplayStatics.UnloadStreamLevel` _stagename true)
  (bind _output_get (set `self.StageName` (`KismetStringLibrary.Conv_StringToName` (`KismetStringLibrary.Concat_StrStr` (`KismetStringLibrary.Left` _returnvalue 5) (`KismetStringLibrary.Conv_IntToString` (+ (`KismetStringLibrary.Conv_StringToInt` (`KismetStringLibrary.RightChop` _returnvalue 5)) 1))))))
  (`GameplayStatics.LoadStreamLevel` _output_get true true)
  (`self.SetAwardTransform`))

(event `CreateUi`
  ;[1 1 1] CreateUi
  (bind _returnvalue (`|CreateWidget` "/Game/UI/W_Play.W_Play_C"))
  (`UserWidget.AddToViewport` _returnvalue 0))

(event `InitialGameInstance`
  (bind _asaward_game_instace (cast `/Game/BP/AwardGameInstace` (`GameplayStatics.GetGameInstance`) :!pure true))
  ;[1 1 1] initialize
  (set `self.AGIVar` _asaward_game_instace)
  (set `/Game/BP/AwardGameInstace.Life` 0 _asaward_game_instace)
  (set `/Game/BP/AwardGameInstace.IsClear` false _asaward_game_instace)
  (set `/Game/BP/AwardGameInstace.Item` 0 _asaward_game_instace)
  (set `/Game/BP/AwardGameInstace.Second` 0 _asaward_game_instace)
  (set `/Game/BP/AwardGameInstace.Minute` 0 _asaward_game_instace))

(event `Time`
  ;[1 1 1] CountUp
  (`KismetSystemLibrary.K2_SetTimerDelegate` (delegate `CountUp`) 1.0 true))

(event `CountUp`
  (bind _agivar (`self.AGIVar`))
  (bind _second (`/Game/BP/AwardGameInstace.Second` _agivar))
  ;[1 1 1] CountUp
  (if (not (and (== (`/Game/BP/AwardGameInstace.Second` _agivar) 59) (== (`/Game/BP/AwardGameInstace.Minute` _agivar) 99)))
    (set `/Game/BP/AwardGameInstace.Second` (+ _second 1) _agivar)
    (if (> _second 59)
      (set `/Game/BP/AwardGameInstace.Minute` (+ (`/Game/BP/AwardGameInstace.Minute` _agivar) 1) _agivar)
      (set `/Game/BP/AwardGameInstace.Second` 0 _agivar))))

(fn `SetAwardTransform`
  (`self.K2_SetActorTransform` (`GameplayStatics.GetPlayerPawn` 0) (`self.GetTransform` (`self.K2_FindPlayerStart` null)) false false))

(fn `UserConstructionScript`)