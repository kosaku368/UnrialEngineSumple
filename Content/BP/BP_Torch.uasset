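; Torch actor with a fire particle system and point light whose color signals goal and game-clear state.
; The construction script tints both flame and light blue when the torch is flagged as IsGoal.
; On BeginPlay, it turns both red if the level is "End" and the game instance's IsClear flag is false.
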(event `self.ReceiveBeginPlay`
  (bind _returnvalue (`GameplayStatics.GetCurrentLevelName` true))
  (if (and (`KismetStringLibrary.EqualEqual_StrStr` _returnvalue "End") (not (`/Game/BP/AwardGameInstace.IsClear` (cast `/Game/BP/AwardGameInstace` (`GameplayStatics.GetGameInstance`) :!pure true))))
    (`FXSystemComponent.SetColorParameter` (`self.ParticleSystem`) "FireColor" (struct :`R` 1.0 :`A` 1.0))
    (`LightComponent.SetLightColor` (`self.PointLight`) (struct :`R` 1.0 :`A` 1.0) true)))

(fn `UserConstructionScript`
  (if (`self.isGoal`)
    (`FXSystemComponent.SetColorParameter` (`self.ParticleSystem`) "FireColor" (struct :`G` 0.25 :`B` 1.0 :`A` 1.0))
    (`LightComponent.SetLightColor` (`self.PointLight`) (struct :`G` 0.25 :`B` 1.0 :`A` 1.0) true)))